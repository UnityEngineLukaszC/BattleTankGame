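; Tank wheel actor that animates its suspension spring and arm from the height difference between the Wheel and Spring components.
; The Wheel component is hidden at BeginPlay without affecting its children, so it serves as an invisible position reference.
; Each tick, that vertical offset drives the spring's "Tension" morph target and sets the IKPos transform on the suspension arm's AnimBP.
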(event `self.ReceiveBeginPlay`
  (`SceneComponent.SetVisibility` (`self.Wheel`) false false))

(event `self.ReceiveActorBeginOverlap`
  (params (OtherActor :type "Actor Object Reference")))

(event `self.ReceiveTick`
  (params (DeltaSeconds :type "Float (single-precision)"))
  (bind _z (.z (- (`SceneComponent.K2_GetComponentLocation` (`self.Wheel`)) (`SceneComponent.K2_GetComponentLocation` (`self.Spring`)))))
  (`SkeletalMeshComponent.SetMorphTarget` (`self.SuspensionSpring`) "Tension" (`KismetMathLibrary.MapRangeUnclamped` (`KismetMathLibrary.Abs` _z) 50.0 100.0 0.0 1.0) true)
  (bind _assuspension_arm_final_anim_bp (cast `/Game/Experiment/Final/SuspensionArmFinal_AnimBP` (`SkeletalMeshComponent.GetAnimInstance` (`self.SuspensionArm`))))
  (set `/Game/Experiment/Final/SuspensionArmFinal_AnimBP.IKPos` (`KismetMathLibrary.MakeTransform` (`KismetMathLibrary.MakeVector` 20.0 0.0 (+ _z 10.0))) _assuspension_arm_final_anim_bp))

(fn `UserConstructionScript`)